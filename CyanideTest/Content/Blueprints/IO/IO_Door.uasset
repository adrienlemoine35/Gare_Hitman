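; Interactive swinging door that AI pawns open on overlap and the player toggles, with an optional key lock marked by a decal.
; Front and back triggers set swing direction and show player prompts reflecting key count.
; Timelines drive the yaw, while a door-state enum controls which triggers have collision during and after movement.
; Opening clears the key requirement without checking keys; key count only affects the prompt here.
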(event `OpenDoor`
  (params (bFront :type Boolean))
  ;[1 1 1] Move the door front or back and reactivate triggers
  (if (`self.bKeyRequired`)
    (`SceneComponent.SetHiddenInGame` (`self.Decal`) true false)
    (set `self.bKeyRequired` false))
  (switch `/Game/Blueprints/IO/Enum_DoorState` (`self.DoorState`)
    (:`NewEnumerator0`
      (set `self.DoorState` (select `bool` bFront :`false` "NewEnumerator2" :`true` "NewEnumerator1" :!type "/Game/Blueprints/IO/Enum_DoorState Enum"))
      (`self.TriggerStop`)
      (bind (_direction _opendoor) (`Timeline|Open` :!via `PlayFromStart`)
        (:`Update`
          (`SceneComponent.K2_SetRelativeRotation` (`self.DoorIO`) (`KismetMathLibrary.MakeRotator` 0.0 0.0 (* _opendoor (select `bool` bFront :`false` 1.0 :`true` -1.0 :!type "Float (single-precision)") 90.0)) false false))
        (:`Finished`
          (`self.TriggerStart`))))))

(event `CloseDoor`
  (bind _doorstate (`self.DoorState`))
  ;[1 1 1] Move the door and reactivate trigger after rotation
  (switch `/Game/Blueprints/IO/Enum_DoorState` _doorstate
    (:`NewEnumerator1`
      _)
    (:`NewEnumerator2`
      _))
  (set `self.CloseWay` (select `/Game/Blueprints/IO/Enum_DoorState` _doorstate :`NewEnumerator1` -1.0 :`NewEnumerator2` 1.0 :!type "Float (single-precision)"))
  (set `self.DoorState` "NewEnumerator0")
  (`self.TriggerStop`)
  (bind (_direction _opendoor) (`Timeline|Timeline_0` :!via `PlayFromStart`)
    (:`Update`
      (`SceneComponent.K2_SetRelativeRotation` (`self.DoorIO`) (`KismetMathLibrary.MakeRotator` 0.0 0.0 (* _opendoor (`self.CloseWay`) 90.0)) false false))
    (:`Finished`
      (`self.TriggerStart`))))

(event `self.FrontTrigger.OnComponentBeginOverlap`
  (params (OverlappedComponent :type "PrimitiveComponent Object Reference") (OtherActor :type "Actor Object Reference") (OtherComp :type "PrimitiveComponent Object Reference") (OtherBodyIndex :type Integer) (bFromSweep :type Boolean) (SweepResult :type "HitResult Structure (by ref)"))
  (bind _textfront (`self.TextFront`))
  ;[1 1 1] Open door front
  (`|ExecutionSequence`
    (:`then_0`
      (cast `/Game/Blueprints/AI/AI_Pawn_BP` OtherActor)
      (`self.OpenDoor` true))
    (:`then_1`
      (cast `/Game/Blueprints/BasePlayer_Pawn` OtherActor)
      (if (`|EnumEquality` (`self.DoorState`) "NewEnumerator0")
        (`SceneComponent.SetHiddenInGame` _textfront false false)
        (`self.SetOpenMessage` _textfront)))))

(event `self.BackTrigger.OnComponentBeginOverlap`
  (params (OverlappedComponent :type "PrimitiveComponent Object Reference") (OtherActor :type "Actor Object Reference") (OtherComp :type "PrimitiveComponent Object Reference") (OtherBodyIndex :type Integer) (bFromSweep :type Boolean) (SweepResult :type "HitResult Structure (by ref)"))
  (bind _textback (`self.TextBack`))
  ;[1 1 1] Open door back
  (`|ExecutionSequence`
    (:`then_0`
      (cast `/Game/Blueprints/AI/AI_Pawn_BP` OtherActor)
      (`self.OpenDoor` false))
    (:`then_1`
      (cast `/Game/Blueprints/BasePlayer_Pawn` OtherActor)
      (if (`|EnumEquality` (`self.DoorState`) "NewEnumerator0")
        (`SceneComponent.SetHiddenInGame` _textback false false)
        (`self.SetOpenMessage` _textback)))))

(event `self.FrontTrigger.OnComponentEndOverlap`
  (params (OverlappedComponent :type "PrimitiveComponent Object Reference") (OtherActor :type "Actor Object Reference") (OtherComp :type "PrimitiveComponent Object Reference") (OtherBodyIndex :type Integer))
  ;[1 1 1] Open door front
  (cast `/Game/Blueprints/BasePlayer_Pawn` OtherActor)
  (`SceneComponent.SetHiddenInGame` (`self.TextFront`) true false))

(event `self.BackTrigger.OnComponentEndOverlap`
  (params (OverlappedComponent :type "PrimitiveComponent Object Reference") (OtherActor :type "Actor Object Reference") (OtherComp :type "PrimitiveComponent Object Reference") (OtherBodyIndex :type Integer))
  ;[1 1 1] Open door back
  (cast `/Game/Blueprints/BasePlayer_Pawn` OtherActor)
  (`SceneComponent.SetHiddenInGame` (`self.TextBack`) true false))

(fn `OpenAndCloseDoorPlayer`
  (`|ExecutionSequence`
    (:`then_0`
      (switch `/Game/Blueprints/IO/Enum_DoorState` (`self.DoorState`)
        (:`NewEnumerator0`
          (`self.OpenDoor` (`PrimitiveComponent.IsOverlappingActor` (`self.FrontTrigger`) (`GameplayStatics.GetPlayerPawn` 0))))
        (:`NewEnumerator1`
          (`self.CloseDoor` :!label _label)
          (`SceneComponent.SetHiddenInGame` (`self.TextFront`) true false)
          (`SceneComponent.SetHiddenInGame` (`self.TextBack`) true false))
        (:`NewEnumerator2`
          (goto _label))))
    (:`then_1`
      (if (`self.bKeyRequired`)
        (set `self.bKeyRequired` false)))))

(fn `SetOpenMessage`
  (params (Text :type "TextRenderComponent Object Reference"))
  (if (`self.bKeyRequired`)
    (bind _asbase_player_pawn (cast `/Game/Blueprints/BasePlayer_Pawn` (`GameplayStatics.GetPlayerPawn` 0)))
    (`TextRenderComponent.K2_SetText` Text (select `bool` (> (`/Game/Blueprints/BasePlayer_Pawn.nb_Key` _asbase_player_pawn) 0) :`false` (`self.TextKeyNeeded`) :`true` (`self.TextOpen`)))
    (else
      (`TextRenderComponent.K2_SetText` Text (`self.TextOpen`)))))

(fn `TriggerStart`
  (bind _backtrigger (`self.BackTrigger`))
  (bind _doorstate (`self.DoorState`))
  ;[1 1 1] Enable trigger depending on door state
  (switch `/Game/Blueprints/IO/Enum_DoorState` _doorstate
    (:`NewEnumerator0`
      (`PrimitiveComponent.SetCollisionEnabled` _backtrigger "QueryOnly")
      (`PrimitiveComponent.SetCollisionEnabled` (`self.FrontTrigger`) "QueryOnly"))
    (:`NewEnumerator1`
      (`PrimitiveComponent.SetCollisionEnabled` (select `/Game/Blueprints/IO/Enum_DoorState` _doorstate :`NewEnumerator1` _backtrigger :`NewEnumerator2` (`self.FrontTrigger`) :!type "PrimitiveComponent Object Reference") "QueryOnly" :!label _label))
    (:`NewEnumerator2`
      (goto _label))))

(fn `TriggerStop`
  (bind _doorstate (`self.DoorState`))
  ;[1 1 1] Remove collisions for triggers
  (switch `/Game/Blueprints/IO/Enum_DoorState` _doorstate
    (:`NewEnumerator1`
      _)
    (:`NewEnumerator2`
      _))
  (`PrimitiveComponent.SetCollisionEnabled` (select `/Game/Blueprints/IO/Enum_DoorState` _doorstate :`NewEnumerator1` (`self.FrontTrigger`) :`NewEnumerator2` (`self.BackTrigger`)) "NoCollision"))

(fn `UserConstructionScript`
  (bind _bkeyrequired (`self.bKeyRequired`))
  (bind _decal (`self.Decal`))
  ;[1 1 1] Door need key or not
  (`parent.UserConstructionScript`)
  (`SceneComponent.SetHiddenInGame` _decal (not _bkeyrequired) false)
  (`SceneComponent.SetVisibility` _decal _bkeyrequired false))