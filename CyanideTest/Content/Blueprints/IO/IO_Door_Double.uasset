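; Double-door variant of an interactive IO door that adds a second leaf following the parent's DoorIO rotation.
; While its gate is open, Tick sets the StaticMesh relative rotation from DoorIO, offsetting and negating yaw to mirror the swing.
; TriggerStop opens that gate and TriggerStart closes it, each after calling the parent implementation.
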(event `self.ReceiveTick`
  (params (DeltaSeconds :type "Float (single-precision)"))
  ;[1 1 1] Update door rotation
  (`/Engine/EditorBlueprintResources/StandardMacros.Gate` true :!label _label
    (:`Exit`
      (`SceneComponent.K2_SetRelativeRotation` (`self.StaticMesh`) (`KismetMathLibrary.MakeRotator` (.roll (`SceneComponent.RelativeRotation` (`self.DoorIO`))) (.pitch (`SceneComponent.RelativeRotation` (`self.DoorIO`))) (* (+ (.yaw (`SceneComponent.RelativeRotation` (`self.DoorIO`))) 180.0) -1.0)) false false))))

(event `self.TriggerStop`
  ;[1 1 1] Update door rotation
  (`parent.TriggerStop`)
  (goto _label :!via `Open`))

(event `self.TriggerStart`
  ;[1 1 1] Update door rotation
  (`parent.TriggerStart`)
  (goto _label :!via `Close`))

(fn `UserConstructionScript`
  (`parent.UserConstructionScript`))