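; Dialogue actor that plays a timed exchange between AI speakers when the player enters its activation volume.
; It steps through the sentences with delays scaled to text length, moving a color-tinted icon above the current speaker.
; The player pawn receives the dialogue on overlap and clears it on exit or completion.
; Speakers' life and AI state gate the start and are polled on Tick to abort the conversation.
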(event `self.ReceiveBeginPlay`
  (bind _volumeactivation (`self.VolumeActivation`))
  (`/Engine/EditorBlueprintResources/StandardMacros.IsValid` _volumeactivation
    (:`Is Valid`
      (add `self.OnActorBeginOverlap` _volumeactivation (delegate `StartOverlap`))
      (add `self.OnActorEndOverlap` _volumeactivation (delegate `HideDial`)))))

(event `HideDial` :!signature `self.OnActorEndOverlap`
  (params (OverlappedActor :type "Actor Object Reference") (OtherActor :type "Actor Object Reference"))
  (bind _asbase_player_pawn (cast `/Game/Blueprints/BasePlayer_Pawn` (`GameplayStatics.GetPlayerPawn` 0) :!label _label))
  (`/Game/Blueprints/BasePlayer_Pawn.SetDialogue` _asbase_player_pawn null))

(event `StartOverlap` :!signature `self.OnActorBeginOverlap`
  (params (OverlappedActor :type "Actor Object Reference") (OtherActor :type "Actor Object Reference"))
  (cast `/Game/Blueprints/BasePlayer_Pawn` OtherActor)
  (if (`self.bDialogStarted`)
    (if (not (`self.bDialogEnded`))
      (bind _asbase_player_pawn (cast `/Game/Blueprints/BasePlayer_Pawn` (`GameplayStatics.GetPlayerPawn` 0) :!label _label_2))
      (`/Game/Blueprints/BasePlayer_Pawn.SetDialogue` _asbase_player_pawn self)
      (`SceneComponent.SetHiddenInGame` (`self.DialIcon`) false false))
    (else
      (`self.StartDialogue` false)
      (goto _label_2))))

(event `DialogueStart`
  (params (bOverrideConditions :type Boolean))
  (bind _indexdial (`self.IndexDial`))
  (bind _returnvalue (`KismetArrayLibrary.Array_Length` (`self.Dialogues`)))
  (bind _output (`|GetArrayItem` (`self.Dialogues`) _indexdial))
  ;[1 1 1] Start Dial then loop if they're still a sentence to play
  (if bOverrideConditions
    (if (!= _returnvalue 0) :!label _label_3
      (set `self.IndexDial` 0)
      (if (< _indexdial _returnvalue) :!label _label_4
        (set `self.CurrentSentence` _output)
        (`self.UpdateIcon`)
        (`KismetSystemLibrary.Delay` (`self.GetSentenceDelay` _output))
        (if (not (`self.bDialogStop`))
          (`/Engine/EditorBlueprintResources/StandardMacros.IncrementInt` (`self.IndexDial`)
            (:`  `
              (goto _label_4))))
        (else
          (`self.EndDialogEvent` :!label _label_5)
          (set `self.bDialogEnded` true)
          (`SceneComponent.SetHiddenInGame` (`self.DialIcon`) true false)
          (goto _label))))
    (elif (`self.CanStartDial`)
      (set `self.bDialogStarted` true)
      (goto _label_3)
      (else
        (bind _ai (break `/Game/Blueprints/Features/Dialogue_Sentence_Struct` (stale `self.ReceiveTick` _array_element)))
        ;[1 1 1] Tick to check if talkers are always alive
        (if (or (not (`/Game/Blueprints/AI/AI_Pawn_BP.isAlive` _ai)) (> (`/Game/Blueprints/AI/AI_Pawn_BP.AIState` _ai) 0)) :!label _label_6
          (set `self.bDialogStop` true)
          (goto _label_5))))))

(event `self.ReceiveTick`
  (params (DeltaSeconds :type "Float (single-precision)"))
  ;[1 1 1] Tick to check if talkers are always alive
  (if (not (`self.bDialogStop`))
    (`KismetSystemLibrary.Delay` 0.2)
    (for _array_element (`self.Dialogues`)
      (goto _label_6))))

(fn `CanStartDial`
  (returns (bCanStart :type Boolean))
  ;[1 1 1] Check if the dial can be played
  (for _array_element (`self.Dialogues`)
    (bind _ai (break `/Game/Blueprints/Features/Dialogue_Sentence_Struct` _array_element))
    (`/Engine/EditorBlueprintResources/StandardMacros.IsValid` _ai
      (:`Is Valid`
        (if (or (not (`/Game/Blueprints/AI/AI_Pawn_BP.isAlive` _ai)) (> (`/Game/Blueprints/AI/AI_Pawn_BP.AIState` _ai) 0))
          (return false)))
      (:`Is Not Valid`
        (return false))))
  (return true))

(fn `GetSentenceDelay`
  (params (Sentence :type "/Game/Blueprints/Features/Dialogue_Sentence_Struct Structure"))
  (returns (Delay :type "Float (double-precision)"))
  ;[1 1 1] Calculate sentence delay based on sentence lenght
  (return (* (`KismetStringLibrary.Len` (`.Sentence_5_BE64A1C6420632608746C49C36770058` (break `/Game/Blueprints/Features/Dialogue_Sentence_Struct` Sentence))) 0.15)))

(fn `StartDialogue`
  (params (bOverrideConditions :type Boolean))
  ;[1 1 1] Start Dialogue
  (`self.DialogueStart` bOverrideConditions))

(fn `UpdateIcon`
  (bind _ai (break `/Game/Blueprints/Features/Dialogue_Sentence_Struct` (`self.CurrentSentence`)))
  (`MaterialInstanceDynamic.SetVectorParameterValue` (`self.DynMat`) "DialColor" (`KismetMathLibrary.Conv_ColorToLinearColor` (`/Game/Blueprints/AI/AI_Pawn_BP.DialColor` _ai)))
  (`SceneComponent.K2_SetWorldLocation` (`self.DialIcon`) (+ (`self.K2_GetActorLocation` _ai) (0.0 0.0 120.0)) false false))

(fn `UserConstructionScript`
  (bind _returnvalue (`PrimitiveComponent.CreateDynamicMaterialInstance` (`self.DialIcon`) 0 (`PrimitiveComponent.GetMaterial` (`self.DialIcon`) 0)))
  (set `self.DynMat` _returnvalue))