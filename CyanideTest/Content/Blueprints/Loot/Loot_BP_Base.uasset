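; Base Blueprint for loot objects, with a mesh, a collision box and a taken state.
; BeginPlay creates a dynamic material on the mesh, whose activation parameter ActivationFeedBack toggles to show feedback.
; GetLoot marks the loot taken, hides the mesh, disables box collision and calls the LootTaken event dispatcher.
; HideObject toggles mesh visibility and switches box collision between none and query-only.
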(event `self.ReceiveBeginPlay`
  (bind _mesh (`self.Mesh`))
  ;[1 1 1] Create the dynamic material
  (bind _returnvalue (`PrimitiveComponent.CreateDynamicMaterialInstance` _mesh 0 (`PrimitiveComponent.GetMaterial` _mesh 0)))
  (set `self.DynamicMat` _returnvalue))

(fn `ActivationFeedBack`
  (params (bActivate :type Boolean))
  (bind _dynamicmat (`self.DynamicMat`))
  ;[1 1 1] Change material based on Feedback changes
  (`/Engine/EditorBlueprintResources/StandardMacros.IsValid` _dynamicmat
    (:`Is Valid`
      (if bActivate
        (`MaterialInstanceDynamic.SetScalarParameterValue` _dynamicmat "LootActivationParam" 1.0)
        (else
          (`MaterialInstanceDynamic.SetScalarParameterValue` _dynamicmat "LootActivationParam" 0.0))))))

(fn `getLoot`
  ;[1 1 1] Loot is taken
  (set `self.bTaken` true)
  (`PrimitiveComponent.SetCollisionEnabled` (`self.Box`) "NoCollision")
  (`SceneComponent.SetHiddenInGame` (`self.Mesh`) true false)
  (`self.ED_LootTaken`))

(fn `HideObject`
  (params (bHide :type Boolean))
  (`SceneComponent.SetHiddenInGame` (`self.Mesh`) bHide false)
  (`PrimitiveComponent.SetCollisionEnabled` (`self.Box`) (select `bool` bHide :`false` "QueryOnly" :`true` "NoCollision" :!type "ECollisionEnabled Enum")))

(fn `UserConstructionScript`)