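; Loot Blueprint for "Aims" that inherits from a parent class and keeps a flag for whether it can be removed.
; Every Tick it casts the first player pawn to BasePlayer_Pawn and sets CanRemove true only when that pawn's ToolBox is true and one specific SkillSelected enum value is active.
; Its construction script only calls the parent's.
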(event `self.ReceiveTick`
  (params (DeltaSeconds :type "Float (single-precision)"))
  (bind _asbase_player_pawn (cast `/Game/Blueprints/BasePlayer_Pawn` (`GameplayStatics.GetPlayerPawn` 0)))
  (if (and (`/Game/Blueprints/BasePlayer_Pawn.ToolBox` _asbase_player_pawn) (`|EnumEquality` (`/Game/Blueprints/BasePlayer_Pawn.SkillSelected` _asbase_player_pawn) "NewEnumerator5"))
    (set `self.CanRemove` true)
    (else
      (set `self.CanRemove` false))))

(fn `UserConstructionScript`
  (`parent.UserConstructionScript`))