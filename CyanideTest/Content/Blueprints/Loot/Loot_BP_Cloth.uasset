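; Cloth loot actor that tints its mesh blue, red or grey according to its ColorType.
; Every Tick, a switch on ColorType writes the matching color into the "Color" vector parameter on the Mesh materials, so the tint is reapplied each frame rather than set once.
; The construction script only calls the parent's, and the BeginPlay and overlap events are unused.
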(event `self.ReceiveTick`
  (params (DeltaSeconds :type "Float (single-precision)"))
  (bind _mesh (`self.Mesh`))
  (switch `/Game/Blueprints/AI/E_AIColor` (`self.ColorType`)
    (:`NewEnumerator0`
      (`MeshComponent.SetVectorParameterValueOnMaterials` _mesh "Color" (`KismetMathLibrary.Conv_LinearColorToVector` (struct :`B` 1.0 :`A` 1.0))))
    (:`NewEnumerator1`
      (`MeshComponent.SetVectorParameterValueOnMaterials` _mesh "Color" (`KismetMathLibrary.Conv_LinearColorToVector` (struct :`R` 1.0 :`A` 1.0))))
    (:`NewEnumerator2`
      (`MeshComponent.SetVectorParameterValueOnMaterials` _mesh "Color" (`KismetMathLibrary.Conv_LinearColorToVector` (struct :`R` 0.450786 :`G` 0.40724 :`B` 0.361307 :`A` 1.0))))))

(fn `UserConstructionScript`
  (`parent.UserConstructionScript`))