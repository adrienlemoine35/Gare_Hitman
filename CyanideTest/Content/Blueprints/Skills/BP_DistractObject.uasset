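; BP_DistractObject is a bottle skill object that smashes on impact to make a noise that distracts AI.
; On the first component hit, it applies radius damage to its destructible mesh and plays a smash sound.
; It then sends a sound target at the bottle's location to every AI_Pawn_BP in the level.
; A gate closes afterward to block repeat hits, and the actor destroys itself after a short delay.
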(event `self.ReceiveBeginPlay`)

(event `self.BottleDistract_DM.OnComponentHit`
  (params (HitComponent :type "PrimitiveComponent Object Reference") (OtherActor :type "Actor Object Reference") (OtherComp :type "PrimitiveComponent Object Reference") (NormalImpulse :type "Vector Structure") (Hit :type "HitResult Structure (by ref)"))
  (bind _returnvalue (`SceneComponent.K2_GetComponentLocation` (`self.BottleDistract_DM`)))
  ;[1 1 1] Add stimuli to AI on bottle hit
  (`/Engine/EditorBlueprintResources/StandardMacros.Gate` false :!label _label
    (:`Exit`
      (`DestructibleComponent.ApplyRadiusDamage` (`self.BottleDistract_DM`) 50.0 _returnvalue 50.0 50.0 true)
      (`GameplayStatics.PlaySoundAtLocation` "/Game/Blueprints/Sounds/BottleSmash_Cue.BottleSmash_Cue" _returnvalue)
      (bind _outactors (`GameplayStatics.GetAllActorsOfClass` "/Game/Blueprints/AI/AI_Pawn_BP.AI_Pawn_BP_C"))
      (for _array_element _outactors
        (`/Game/Blueprints/AI/AI_Pawn_BP.CreateSoundTarget` _array_element 150.0 _returnvalue))
      (`|ExecutionSequence`
        (:`then_0`
          (goto _label :!via `Close`))
        (:`then_1`
          (`KismetSystemLibrary.Delay` 1.0)
          (`self.K2_DestroyActor`))))))

(fn `UserConstructionScript`)