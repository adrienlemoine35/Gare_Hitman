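; AI patrol point actor that links to a next point and visualizes the patrol route through its construction script.
; InitDisplay aims and stretches an arrow toward NextPatrolPoint and shows a billboard and facing arrow only when WaitTime is positive.
; It recurses along the chain, passing on the patrol color for dynamic materials, until the link is invalid or returns to the start point.
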(fn `ChangeDisplayColor`
  (bind _returnvalue (`PrimitiveComponent.CreateDynamicMaterialInstance` (`self.ArrowNextPoint`) 0 (`self.MatInstColor`)))
  (bind _output_get (set `self.MatInstColor` _returnvalue))
  (`MaterialInstanceDynamic.SetVectorParameterValue` _output_get "PatrolColorParameter" (`self.PatrolColor`))
  (bind _returnvalue_2 (`PrimitiveComponent.CreateDynamicMaterialInstance` (`self.MeshPP`) 0 (`self.MatInstColorArrow`)))
  (bind _output_get_2 (set `self.MatInstColorArrow` _returnvalue_2))
  (`MaterialInstanceDynamic.SetVectorParameterValue` _output_get_2 "PatrolColorParameter" (`self.PatrolColor`)))

(fn `InitDisplay`
  (params (StartPoint :type "/Game/Blueprints/AI/AI_Point_Patrol_BP Object Reference") (Color :type "LinearColor Structure"))
  (bind _arrownextpoint (`self.ArrowNextPoint`))
  (bind _nextpatrolpoint (`self.NextPatrolPoint`))
  (bind _nextpatrolpoint_2 (`self.NextPatrolPoint`))
  (`|ExecutionSequence`
    (:`then_0`
      (set `self.PatrolColor` Color)
      (`self.ChangeDisplayColor`)
      (`/Engine/EditorBlueprintResources/StandardMacros.IsValid` _nextpatrolpoint
        (:`Is Valid`
          (`SceneComponent.K2_SetWorldRotation` _arrownextpoint (`KismetMathLibrary.FindLookAtRotation` (`self.K2_GetActorLocation` self) (`self.K2_GetActorLocation` _nextpatrolpoint)) false false)
          (`SceneComponent.SetWorldScale3D` _arrownextpoint (`KismetMathLibrary.MakeVector` (/ (`self.GetDistanceTo` self _nextpatrolpoint) 80.0) 0.2 0.2)))))
    (:`then_1`
      (if (> (`self.WaitTime`) 0.0)
        (`SceneComponent.SetVisibility` (`self.Billboard`) true false)
        (`SceneComponent.SetVisibility` (`self.Arrow`) true false)
        (else
          (`SceneComponent.SetVisibility` (`self.Arrow`) false false)
          (`SceneComponent.SetVisibility` (`self.Billboard`) false false))))
    (:`then_2`
      (if (and (!= _nextpatrolpoint_2 StartPoint) (`KismetSystemLibrary.IsValid` _nextpatrolpoint_2))
        (`self.InitDisplay` _nextpatrolpoint_2 StartPoint (`self.PatrolColor`))))))

(fn `UserConstructionScript`
  (`parent.UserConstructionScript`)
  (`self.InitDisplay` self (`self.PatrolColor`)))