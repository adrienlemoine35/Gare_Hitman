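; Stealth enemy AI pawn that patrols and detects the player, but ignores players matching its color.
; Nearby, Tick turns sight perception, weighted by distance and angle, into progression through Patrol, Suspicious, Search and Alert using tuning data.
; Noise and touch also raise detection, feeding follow, check and search targets alongside the controller's behavior tree.
; It also drains the player's gauge in Alert, carries vial/key loot, and ragdolls and dissolves when killed.
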(event `self.ReceiveTick`
  (params (DeltaSeconds :type "Float (single-precision)"))
  ;[1 1 1] IA Behavior
  ;;[1 1 1] UpdateDetection
  (if (and (`self.Activated`) (`self.isAlive`) (`self.IATickOptim`) (`self.bCanSeePlayerColor`))
    (switch `/Game/Blueprints/AI/E_AI_State` (`self.AIState`)
      (:`NewEnumerator0`
        _)
      (:`NewEnumerator1`
        _)
      (:`NewEnumerator2`
        _)
      (:`NewEnumerator3`
        (`self.DecreasePlayerGauge` DeltaSeconds)))
    (`self.UpdateDetectedActor`)
    (`|ExecutionSequence`
      (:`then_0`
        (`self.UpdateDetection` DeltaSeconds)
        (`self.UpdateStateChange`)
        (switch `/Game/Blueprints/AI/E_AI_State` (`self.AIState`)
          (:`NewEnumerator1`
            _)
          (:`NewEnumerator2`
            _)
          (:`NewEnumerator3`
            _))
        (`/Engine/EditorBlueprintResources/StandardMacros.IsValid` (`self.LastActorSeen`)
          (:`Is Valid`
            (set `self.TargetToFollow` (`GameplayStatics.GetPlayerPawn` 0)))))
      (:`then_1`
        (`/Engine/EditorBlueprintResources/StandardMacros.IsValid` (`self.LastActorSeen`)
          (:`Is Valid`
            (`KismetSystemLibrary.RetriggerableDelay` (`self.OmniScienceTime`))
            (`self.UpdateLastLocation`)
            (`self.GenerateTargetToCheck` (`self.PossiblePlayerTransform`))
            (set `self.TargetToFollow` null)
            (`KismetSystemLibrary.PrintString` "ClearTarget" true true (struct :`R` 1.0 :`G` 0.049951 :`A` 1.0) 5.0)))))))

(event `self.ReceiveBeginPlay`
  ;[1 1 1] IA Behavior
  ;;[1 1 1] Initialization
  (`self.ChangeAIState` "NewEnumerator0")
  (`self.InitAI`)
  (`self.InitPickPocket`)
  (bind _asai_controller_bp (cast `/Game/Blueprints/AI/AI_Controller_BP` (`self.GetController`)))
  (`/Game/Blueprints/AI/AI_Controller_BP.RunBT` _asai_controller_bp))

(event `SearchPointChecked`
  ;[1 1 1] IA Behavior
  ;;[1 1 1] BT Notification
  (`self.ForceState` "NewEnumerator0"))

(event `SeeTargetChecked`
  ;[1 1 1] IA Behavior
  ;;[1 1 1] BT Notification
  (set `self.TargetToCheck` null)
  (switch `/Game/Blueprints/AI/E_AI_State` (`self.AIState`)
    (:`NewEnumerator1`
      (`self.ForceState` "NewEnumerator0"))
    (:`NewEnumerator2`
      (`self.ForceState` "NewEnumerator2" :!label _label))
    (:`NewEnumerator3`
      (goto _label))))

(event `self.CapsuleComponent.OnComponentHit`
  (params (HitComponent :type "PrimitiveComponent Object Reference") (OtherActor :type "Actor Object Reference") (OtherComp :type "PrimitiveComponent Object Reference") (NormalImpulse :type "Vector Structure") (Hit :type "HitResult Structure (by ref)"))
  ;[1 1 1] IA Behavior
  ;;[1 1 1] Touched by player
  (if (and (`self.Activated`) (`self.isAlive`))
    (cast `/Game/Blueprints/BasePlayer_Pawn` OtherActor)
    (`self.TouchByPlayer`)))

(event `BeginPatrol`
  (params (`Patrol Point` :type "/Game/Blueprints/AI/AI_Point_Patrol_BP Object Reference"))
  ;[1 1 1] IA Behavior
  ;;[1 1 1] Level Event
  (set `self.CurrentPatrolPoint` `Patrol Point`)
  (set `self.isPatrolStarted` true))

(event `ResumePatrol`
  ;[1 1 1] IA Behavior
  ;;[1 1 1] Level Event
  (set `self.isPatrolStarted` true))

(event `PausePatrol`
  ;[1 1 1] IA Behavior
  ;;[1 1 1] Level Event
  (set `self.isPatrolStarted` false))

(event `StartDisolve`
  (bind _mesh (`self.Mesh`))
  ;[1 1 1] IA Behavior
  ;;[1 1 1] Dissolve effect and AI death
  (`KismetSystemLibrary.Delay` 1.25)
  (bind (_direction _disolve) (`Timeline|Timeline_0`)
    (:`Update`
      (`MaterialInstanceDynamic.SetScalarParameterValue` (`self.MatDynamic`) "DisolveAmount" _disolve)
      (`MaterialInstanceDynamic.SetScalarParameterValue` (`self.MatDynamicLogo`) "DisolveAmount" _disolve))
    (:`Finished`
      (`PrimitiveComponent.SetSimulatePhysics` _mesh false)
      (`PrimitiveComponent.SetCollisionEnabled` _mesh "NoCollision")
      (`SceneComponent.SetHiddenInGame` _mesh true false))))

(fn `bCanSeePlayerColor`
  (returns (bCanSee :type Boolean))
  (bind _asbase_player_pawn (cast `/Game/Blueprints/BasePlayer_Pawn` (`GameplayStatics.GetPlayerPawn` 0)))
  (if (== (`KismetMathLibrary.Conv_LinearColorToVector` (`self.GetColor` (`self.AIColor`))) (`KismetMathLibrary.Conv_LinearColorToVector` (`self.GetColor` (`/Game/Blueprints/BasePlayer_Pawn.ColorPerso` _asbase_player_pawn))))
    (return false)
    (else
      (return true))))

(fn `CanDecreaseAIState`
  (returns (bCanDecrease :type Boolean))
  (return (and (== (`KismetArrayLibrary.Array_Length` (`self.PatrolSearch`)) 0) (not (`KismetSystemLibrary.IsValid` (`self.TargetToFollow`))) (not (`KismetSystemLibrary.IsValid` (`self.TargetToCheck`))))))

(fn `ChangeAIState`
  (params (NewState :type "/Game/Blueprints/AI/E_AI_State Enum" :default "NewEnumerator0"))
  ;[1 0 0] Éviter autant que possible de toucher à l'IA
  (bind _output_get (set `self.AIState` NewState))
  (set `CharacterMovementComponent.MaxWalkSpeed` (select `/Game/Blueprints/AI/E_AI_State` _output_get :`NewEnumerator0` 100.0 :`NewEnumerator1` 100.0 :`NewEnumerator2` 200.0 :`NewEnumerator3` 300.0 :!type "Float (single-precision)") (`self.CharacterMovement`))
  (switch `/Game/Blueprints/AI/E_AI_State` _output_get
    (:`NewEnumerator0`
      (`ActorComponent.Activate` (`self.AIPerception`) false))))

(fn `ClampMaxProgression`
  (params (Value :type "Float (double-precision)"))
  (returns (ReturnValue :type "Float (double-precision)"))
  ;[1 0 0] Éviter autant que possible de toucher à l'IA
  (return (`KismetMathLibrary.FClamp` Value 0.0 (`KismetMathLibrary.Conv_IntToDouble` (- (`.LimitUp_19_3FD45F184BE5D7DC2E7946AABDD192B6` (break `/Game/Blueprints/AI/S_AI_StateTransition` (`.Search` (defaults `/Game/Blueprints/AI/AIStateTunning` "/Game/Blueprints/AI/AIStateTunning.AIStateTunning_C")))) 1)))))

(fn `CreateSoundTarget`
  (params (NoiseAmount :type "Float (double-precision)") (Location :type "Vector Structure"))
  ;[1 0 0] Éviter autant que possible de toucher à l'IA
  (if (and (`self.isAlive`) (`self.Activated`) (`|EnumInequality` (`self.AIState`) "NewEnumerator3") (`self.bCanSeePlayerColor`))
    (set `self.StateProgression` (`self.ClampMaxProgression` (+ (`self.StateProgression`) (* NoiseAmount (`KismetMathLibrary.Square` (- 1.0 (/ (`KismetMathLibrary.FClamp` (`KismetMathLibrary.VSize` (* (- Location (`self.K2_GetActorLocation` self)) (1.0 1.0 0.25))) 0.0 2000.0) 2000.0)))))))
    (`self.UpdateStateChange`)
    (switch `/Game/Blueprints/AI/E_AI_State` (`self.AIState`)
      (:`NewEnumerator1`
        _)
      (:`NewEnumerator2`
        _))
    (`self.GenerateTargetToCheck` (`KismetMathLibrary.MakeTransform` Location))))

(fn `CreatSearchPointList`
  (returns (SearchPointList :type "Array of /Game/Blueprints/AI/AI_Point_Search_BP Object Reference"))
  (bind _searchpointlist (`/Game/Blueprints/AI/AIFunctionLibrary.CreateSearchPointListFromContext` self (`self.MaxSearchDistance`) (`self.SearchPointPatrolSize`)))
  (bind _output_get (set `self.PatrolSearch` _searchpointlist))
  (return _output_get))

(fn `DecreasePlayerGauge`
  (params (DTime :type "Float (double-precision)"))
  ;[1 0 0] Éviter autant que possible de toucher à l'IA
  (`/Engine/EditorBlueprintResources/StandardMacros.IsValid` (`self.LastActorSeen`)
    (:`Is Valid`
      (bind _asbase_player_pawn (cast `/Game/Blueprints/BasePlayer_Pawn` (`GameplayStatics.GetPlayerPawn` 0)))
      (set `/Game/Blueprints/BasePlayer_Pawn.alerteGauge` (`KismetMathLibrary.FClamp` (- (`/Game/Blueprints/BasePlayer_Pawn.alerteGauge` _asbase_player_pawn) (* DTime 0.5))) _asbase_player_pawn)
      (`/Game/Blueprints/BasePlayer_Pawn.DecreaseGauge` _asbase_player_pawn))))

(fn `ForceState`
  (params (NewState :type "/Game/Blueprints/AI/E_AI_State Enum" :default "NewEnumerator0"))
  (bind (_patrol _suspicious _search _alert) (defaults `/Game/Blueprints/AI/AIStateTunning` "/Game/Blueprints/AI/AIStateTunning.AIStateTunning_C"))
  (set `self.StateProgression` (`KismetMathLibrary.Conv_IntToDouble` (`.LimitUp_19_3FD45F184BE5D7DC2E7946AABDD192B6` (break `/Game/Blueprints/AI/S_AI_StateTransition` (select `/Game/Blueprints/AI/E_AI_State` NewState :`NewEnumerator0` _patrol :`NewEnumerator1` _suspicious :`NewEnumerator2` _search :`NewEnumerator3` _alert)))))
  (set `self.AIState` NewState)
  (`self.UpdateStateChange`))

(fn `GenerateTargetToCheck`
  (params (Transform :type "Transform Structure"))
  (bind _returnvalue (`|SpawnActorFromClass` "/Script/Engine.TargetPoint" Transform "AlwaysSpawn" "OverrideRootScale" null null))
  (bind _output_get (set `self.TargetToCheck` _returnvalue))
  (`self.SetLifeSpan` _output_get 20.0))

(fn `GetColor`
  (params (Code :type "/Game/Blueprints/AI/E_AIColor Enum" :default "NewEnumerator0"))
  (returns (Color :type "LinearColor Structure"))
  (for _array_element (`self.AIColors`)
    (bind (_code _color) (break `/Game/Blueprints/AI/AI_Color` _array_element))
    (if (`|EnumEquality` _code Code)
      (return _color))))

(fn `IATickOptim`
  (returns (PlayerCloseEnough :type Boolean))
  (return (< (`self.GetDistanceTo` (`GameplayStatics.GetPlayerPawn` 0) self) 2000.0)))

(fn `InitAI`
  (bind _patrolstart (`self.PatrolStart`))
  ;[1 0 0] Éviter autant que possible de toucher à l'IA
  (set `self.CurrentAIStateBar` (defaults `/Game/Blueprints/AI/AIStateTunning` "/Game/Blueprints/AI/AIStateTunning.AIStateTunning_C"))
  (bind _returnvalue (`|CreateWidget` "/Game/Blueprints/UI/UI_AIState.UI_AIState_C"))
  (set `self.DetectionUI` _returnvalue)
  (`UserWidget.AddToViewport` _returnvalue 0)
  (set `/Game/Blueprints/UI/UI_AIState.AIAttached` self _returnvalue)
  (`/Engine/EditorBlueprintResources/StandardMacros.IsValid` _patrolstart
    (:`Is Valid`
      (set `self.CurrentPatrolPoint` _patrolstart)
      (set `self.isPatrolStarted` true))))

(fn `InitPickPocket`
  ;[1 0 0] Éviter autant que possible de toucher à l'IA
  (`|ExecutionSequence`
    (:`then_0`
      (if (`self.bCarryVial`)
        (bind _returnvalue (`|SpawnActorFromClass` "/Game/Blueprints/Loot/Loot_BP_PowerVials.Loot_BP_PowerVials_C" (`SceneComponent.GetSocketTransform` (`self.Mesh`) "VialSocket" "RTS_World") "Undefined" "OverrideRootScale" null null))
        (`self.K2_AttachToComponent` _returnvalue (`self.Mesh`) "VialSocket" "SnapToTarget" "KeepWorld" "KeepWorld" true)
        (set `self.Vial` _returnvalue)))
    (:`then_1`
      (if (`self.bCarryKey`)
        (bind _returnvalue_2 (`|SpawnActorFromClass` "/Game/Blueprints/Loot/Loot_BP_Key.Loot_BP_Key_C" (`SceneComponent.GetSocketTransform` (`self.Mesh`) "KeySocket" "RTS_World") "Undefined" "OverrideRootScale" null null))
        (`self.K2_AttachToComponent` _returnvalue_2 (`self.Mesh`) "KeySocket" "SnapToTarget" "KeepWorld" "KeepWorld" true)
        (set `self.key` _returnvalue_2)))))

(fn `KillAI`
  (params (NormalStab :type "Vector Structure") (bDoNotDisolve :type Boolean))
  (bind _mesh (`self.Mesh`))
  (bind _detectionui (`self.DetectionUI`))
  (bind _detectionui_2 (`self.DetectionUI`))
  (bind _vial (`self.Vial`))
  (bind _key (`self.key`))
  ;[1 0 0] Éviter autant que possible de toucher à l'IA
  (set `self.Activated` false)
  (set `self.AIState` "NewEnumerator0")
  (`/Engine/EditorBlueprintResources/StandardMacros.IsValid` _detectionui_2
    (:`Is Valid`
      (`Widget.RemoveFromParent` _detectionui_2))
    (:`Is Not Valid`
      _))
  (set `self.StateProgression` 0.0)
  (`self.ED_AI_Dead`)
  (`PrimitiveComponent.SetSimulatePhysics` _mesh true)
  (`PrimitiveComponent.SetCollisionEnabled` _mesh "QueryAndPhysics")
  (`PrimitiveComponent.SetCollisionEnabled` (`self.CapsuleComponent`) "NoCollision")
  (if (not bDoNotDisolve)
    (`PrimitiveComponent.AddImpulse` (`self.Mesh`) (* NormalStab 5000.0) "None" true)
    (set `self.isAlive` false)
    (`self.StartDisolve`)
    (`/Engine/EditorBlueprintResources/StandardMacros.IsValid` _detectionui
      (:`Is Valid`
        (`Widget.RemoveFromParent` _detectionui)
        (`|ExecutionSequence`
          (:`then_0`
            (`/Engine/EditorBlueprintResources/StandardMacros.IsValid` _vial
              (:`Is Valid`
                (`self.K2_DestroyActor` _vial))))
          (:`then_1`
            (`/Engine/EditorBlueprintResources/StandardMacros.IsValid` _key
              (:`Is Valid`
                (`self.K2_DestroyActor` _key)))))))))

(fn `SpeedHearingDetectionFactor`
  (returns (F :type "Float (double-precision)"))
  (bind _lastactorseen (`self.LastActorSeen`))
  (bind _returnvalue (`self.GetDistanceTo` _lastactorseen self))
  ;[1 0 0] Éviter autant que possible de toucher à l'IA
  (if (< _returnvalue 1500.0)
    (bind _asbase_player_pawn (cast `/Game/Blueprints/BasePlayer_Pawn` _lastactorseen)
      (:`then`
        (bind _maxwalkspeed (`CharacterMovementComponent.MaxWalkSpeed` (`Character.CharacterMovement` _asbase_player_pawn)))
        (return (* (`KismetMathLibrary.MultiplyMultiply_FloatFloat` (- 1.0 (/ _returnvalue 1500.0)) 2.0) (`KismetMathLibrary.MultiplyMultiply_FloatFloat` (/ (`KismetMathLibrary.FClamp` (`KismetMathLibrary.VSize` (`self.GetVelocity` _asbase_player_pawn)) 0.0 _maxwalkspeed) _maxwalkspeed) 2.0) 10.0)))
      (:`CastFailed`
        _)))
  (return 0.0))

(fn `SpeedVisualDetectionFactor`
  (returns (f :type "Float (double-precision)"))
  (bind _lastactorseen (`self.LastActorSeen`))
  ;[1 0 0] Éviter autant que possible de toucher à l'IA
  (`/Engine/EditorBlueprintResources/StandardMacros.IsValid` _lastactorseen
    (:`Is Valid`
      (return (* (`KismetMathLibrary.MultiplyMultiply_FloatFloat` (- 1.0 (/ (`KismetMathLibrary.FClamp` (`self.GetDistanceTo` _lastactorseen self) 0.0 1500.0) 1500.0)) 2.0) (`KismetMathLibrary.Square` (+ 1.0 (`KismetMathLibrary.FClamp` (`KismetMathLibrary.Dot_VectorVector` (`KismetMathLibrary.Normal` (- (`self.K2_GetActorLocation` _lastactorseen) (`self.K2_GetActorLocation` self))) (`KismetMathLibrary.Normal` (`SceneComponent.GetForwardVector` (`self.CapsuleComponent`))))))))))
    (:`Is Not Valid`
      (return 0.0))))

(fn `TouchByPlayer`
  ;[1 0 0] Éviter autant que possible de toucher à l'IA
  (if (`self.bCanSeePlayerColor`)
    (set `self.StateProgression` (`KismetMathLibrary.Conv_IntToDouble` (`.LimitUp_19_3FD45F184BE5D7DC2E7946AABDD192B6` (break `/Game/Blueprints/AI/S_AI_StateTransition` (`.Alert` (defaults `/Game/Blueprints/AI/AIStateTunning` "/Game/Blueprints/AI/AIStateTunning.AIStateTunning_C"))))))
    (set `self.TargetToFollow` (`GameplayStatics.GetPlayerPawn` 0))
    (`self.ForceState` "NewEnumerator3")))

(fn `UpdateAIState`
  (params (NewState :type "/Game/Blueprints/AI/E_AI_State Enum" :default "NewEnumerator0"))
  (bind (_patrol _suspicious _search _alert) (defaults `/Game/Blueprints/AI/AIStateTunning` "/Game/Blueprints/AI/AIStateTunning.AIStateTunning_C"))
  ;[1 0 0] Éviter autant que possible de toucher à l'IA
  (switch `/Game/Blueprints/AI/E_AI_State` NewState
    (:`NewEnumerator0`
      (set `self.CurrentAIStateBar` _patrol))
    (:`NewEnumerator1`
      (set `self.CurrentAIStateBar` _suspicious))
    (:`NewEnumerator2`
      (set `self.CurrentAIStateBar` _search))
    (:`NewEnumerator3`
      (set `self.CurrentAIStateBar` _alert))))

(fn `UpdateDetectedActor`
  (bind _outactors (`AIPerceptionComponent.GetPerceivedActors` (`self.AIPerception`) "/Script/AIModule.AISense_Sight"))
  ;[1 0 0] Éviter autant que possible de toucher à l'IA
  (`self.ArrayEmpty` _outactors
    (:`Not Empty`
      (bind _filteredarray (`KismetArrayLibrary.FilterArray` _outactors "/Game/Blueprints/AI/SightStimuliSource.SightStimuliSource_C"))
      (set `self.LastActorSeen` (`|GetArrayItem` _filteredarray)))
    (:`Empty`
      (set `self.LastActorSeen` null))))

(fn `UpdateDetection`
  (params (DTime :type "Float (double-precision)"))
  (bind (_state _previousstate _nextstate _limitup _limitdown _speedincreasestatefactor _speeddecreasestatefactor) (break `/Game/Blueprints/AI/S_AI_StateTransition` (`self.CurrentAIStateBar`)))
  (bind _returnvalue (- (`self.StateProgression`) (* DTime _speeddecreasestatefactor)))
  ;[1 0 0] Éviter autant que possible de toucher à l'IA
  (`/Engine/EditorBlueprintResources/StandardMacros.IsValid` (`self.LastActorSeen`)
    (:`Is Valid`
      (set `self.StateProgression` (+ (`self.StateProgression`) (* (`self.SpeedVisualDetectionFactor`) DTime _speedincreasestatefactor))))
    (:`Is Not Valid`
      (if (`self.CanDecreaseAIState`)
        (if (> _returnvalue 0.0)
          (set `self.StateProgression` _returnvalue)
          (else
            (set `self.StateProgression` 0.0)))))))

(fn `UpdateLastLocation`
  (set `self.PossiblePlayerTransform` (`self.GetTransform` (`GameplayStatics.GetPlayerPawn` 0))))

(fn `UpdatePatrolPoint`
  (bind _currentpatrolpoint (`self.CurrentPatrolPoint`))
  (`/Engine/EditorBlueprintResources/StandardMacros.IsValid` _currentpatrolpoint
    (:`Is Valid`
      (set `self.CurrentPatrolPoint` (`/Game/Blueprints/AI/AI_Point_Patrol_BP.NextPatrolPoint` _currentpatrolpoint)))))

(fn `UpdateSearchPoint`
  (returns (SearchPointFound :type "/Game/Blueprints/AI/AI_Point_Search_BP Object Reference"))
  (bind _patrolsearch (`self.PatrolSearch`))
  (`|ExecutionSequence`
    (:`then_0`
      (`/Engine/EditorBlueprintResources/StandardMacros.IsValid` (`self.CurrentSearchPoint`)
        (:`Is Valid`
          (`KismetArrayLibrary.Array_RemoveItem` (`self.PatrolSearch`) (`self.CurrentSearchPoint`)))))
    (:`then_1`
      (if (> (`KismetArrayLibrary.Array_Length` _patrolsearch) 0)
        (set `self.CurrentSearchPoint` (`|GetArrayItem` _patrolsearch))
        (else
          (set `self.CurrentSearchPoint` null))))
    (:`then_2`
      (return (`self.CurrentSearchPoint`)))))

(fn `UpdateStateChange`
  (bind (_state _previousstate _nextstate) (break `/Game/Blueprints/AI/S_AI_StateTransition` (`self.CurrentAIStateBar`)))
  (bind (_state_2 _previousstate_2 _nextstate_2 _limitup _limitdown) (break `/Game/Blueprints/AI/S_AI_StateTransition` (`self.CurrentAIStateBar`)))
  ;[1 0 0] Éviter autant que possible de toucher à l'IA
  (`|ExecutionSequence`
    (:`then_0`
      (if (> (`self.StateProgression`) (`KismetMathLibrary.Conv_IntToDouble` _limitup))
        (`self.UpdateAIState` _nextstate)
        (`self.ChangeAIState` _state :!label _label)))
    (:`then_1`
      (if (< (`self.StateProgression`) (`KismetMathLibrary.Conv_IntToDouble` _limitdown))
        (`self.UpdateAIState` _previousstate)
        (goto _label)))))

(fn `UserConstructionScript`
  (bind _mesh (`self.Mesh`))
  (bind _color (`self.GetColor` (`self.AIColor`)))
  ;[1 0 0] Éviter autant que possible de toucher à l'IA
  (bind _returnvalue (`PrimitiveComponent.CreateDynamicMaterialInstance` _mesh 0 (`self.MatBase`)))
  (set `self.MatDynamic` _returnvalue)
  (bind _returnvalue_2 (`PrimitiveComponent.CreateDynamicMaterialInstance` _mesh 1 (`self.MatLogo`)))
  (set `self.MatDynamicLogo` _returnvalue_2)
  (`MaterialInstanceDynamic.SetVectorParameterValue` (`self.MatDynamic`) "BodyColor" _color)
  (`MaterialInstanceDynamic.SetVectorParameterValue` (`self.MatDynamicLogo`) "BodyColor" _color))