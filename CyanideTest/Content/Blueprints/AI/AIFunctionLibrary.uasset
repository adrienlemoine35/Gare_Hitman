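; AI function library that builds an ordered list of search points around a context actor.
; CreateSearchPointListFromContext gathers AI_Point_Search_BP actors within a straight-line radius and trims them to the requested count before sorting, so the kept points are not necessarily the nearest.
; SortSearchPointFromContext then orders them by path length to the context, nearest first, using a selection sort that recomputes paths on every comparison.
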(fn `CreateSearchPointListFromContext`
  (params (Context :type "Actor Object Reference") (SearchRadius :type "Float (double-precision)") (NumberSearchPoint :type Integer))
  (returns (SearchPointList :type "Array of /Game/Blueprints/AI/AI_Point_Search_BP Object Reference"))
  (locals (PatrolSearch :type "Array of /Game/Blueprints/AI/AI_Point_Search_BP Object Reference") (SearchPatrol :type "Array of /Game/Blueprints/AI/AI_Point_Search_BP Object Reference"))
  (bind _searchpatrol (`local.SearchPatrol`))
  (`|ExecutionSequence`
    (:`then_0`
      (bind _outactors (`GameplayStatics.GetAllActorsOfClass` null "/Game/Blueprints/AI/AI_Point_Search_BP.AI_Point_Search_BP_C"))
      (bind _output_get (set `local.PatrolSearch` _outactors))
      (for _array_element _output_get
        (if (< (`Actor.GetDistanceTo` _array_element Context) SearchRadius)
          (`KismetArrayLibrary.Array_Add` (`local.SearchPatrol`) _array_element)))
      (if (> (`KismetArrayLibrary.Array_Length` _searchpatrol) NumberSearchPoint)
        (`KismetArrayLibrary.Array_Resize` _searchpatrol NumberSearchPoint))
      (bind _newpoints (`self.SortSearchPointFromContext` _searchpatrol Context))
      (set `local.SearchPatrol` _newpoints))
    (:`then_1`
      (return (`local.SearchPatrol`)))))

(fn `GetPathLenBetweenActors`
  (params (Actor1 :type "Actor Object Reference") (Actor2 :type "Actor Object Reference"))
  (returns (NewParam :type "Float (double-precision)"))
  (return (`NavigationSystem.GetPathLength` null (`Actor.K2_GetActorLocation` Actor1) (`Actor.K2_GetActorLocation` Actor2))))

(fn `SortSearchPointFromContext`
  (params (SearchPoints :type "Array of /Game/Blueprints/AI/AI_Point_Search_BP Object Reference") (Context :type "Actor Object Reference"))
  (returns (NewPoints :type "Array of /Game/Blueprints/AI/AI_Point_Search_BP Object Reference"))
  (locals (OldSearchPoints :type "Array of /Game/Blueprints/AI/AI_Point_Search_BP Object Reference") (NewSearchPoints :type "Array of /Game/Blueprints/AI/AI_Point_Search_BP Object Reference") (MinDistPoint :type "/Game/Blueprints/AI/AI_Point_Search_BP Object Reference"))
  (bind _mindistpoint (`local.MinDistPoint`))
  (bind _oldsearchpoints (`local.OldSearchPoints`))
  (set `local.OldSearchPoints` SearchPoints)
  (while (> (`KismetArrayLibrary.Array_Length` _oldsearchpoints) 0)
    (bind _output_get (set `local.MinDistPoint` (`|GetArrayItem` _oldsearchpoints)))
    (for _array_element (`local.OldSearchPoints`)
      (if (< (`self.GetPathLenBetweenActors` _array_element Context) (`self.GetPathLenBetweenActors` _output_get Context))
        (set `local.MinDistPoint` _array_element)))
    (`KismetArrayLibrary.Array_Add` (`local.NewSearchPoints`) _mindistpoint)
    (`KismetArrayLibrary.Array_RemoveItem` (`local.OldSearchPoints`) _mindistpoint))
  (return (`local.NewSearchPoints`)))