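; Objectives manager that runs a sequential quest chain from an ordered Objectives array.
; Construction sets the first objective as current, and BeginPlay hides the Loot_BP_Base actors linked to all later objectives.
; NextQuestStep advances the index, pushes a quest notification to the player pawn's HUDSkill widget and unhides the new objective's loot actor.
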(event `self.ReceiveBeginPlay`
  (for (_array_element _array_index) (`self.Objectives`)
    (if (> _array_index 0)
      (bind _asloot_bp_base (cast `/Game/Blueprints/Loot/Loot_BP_Base` (`.Obj_Location_6_F30DD17A4070D598CE54828DEAA2D0AC` (break `/Game/Blueprints/Struct_Objective` _array_element))))
      (`/Game/Blueprints/Loot/Loot_BP_Base.HideObject` _asloot_bp_base true))))

(fn `AddNotification`
  ;[1 1 1] Add the new objectif
  (bind _asbase_player_pawn (cast `/Game/Blueprints/BasePlayer_Pawn` (`GameplayStatics.GetPlayerPawn` 0)))
  (`/Game/Blueprints/UI/HUD_SkillPower.AddQuestNotif` (`/Game/Blueprints/BasePlayer_Pawn.HUDSkill` _asbase_player_pawn) (`self.CurrentObjective`)))

(fn `NextQuestStep`
  (bind _indexobj (`self.IndexObj`))
  (bind _objectives (`self.Objectives`))
  ;[1 1 1] Set the current objective to the next one
  (if (< _indexobj (`KismetArrayLibrary.Array_Length` _objectives))
    (bind _result (`/Engine/EditorBlueprintResources/StandardMacros.IncrementInt` _indexobj)
      (:`  `
        (bind _output_get (set `self.CurrentObjective` (`|GetArrayItem` _objectives _result)))
        (`self.AddNotification`)
        (bind _asloot_bp_base (cast `/Game/Blueprints/Loot/Loot_BP_Base` (`.Obj_Location_6_F30DD17A4070D598CE54828DEAA2D0AC` (break `/Game/Blueprints/Struct_Objective` _output_get))))
        (`/Game/Blueprints/Loot/Loot_BP_Base.HideObject` _asloot_bp_base false)))))

(fn `UserConstructionScript`
  ;[1 1 1] Set current objective to the first
  (set `self.CurrentObjective` (`|GetArrayItem` (`self.Objectives`))))